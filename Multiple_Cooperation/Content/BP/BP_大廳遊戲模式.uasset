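; Lobby game mode that maintains a list of all connected lobby player controllers (BP_大廳玩家控制器).
; PostLogin adds each controller uniquely; OnLogout removes it and has player controller 0 refresh its player info UI.
; 透過編號尋找玩家控制器 looks up a controller by player code, reading 玩家代號 from each controlled pawn cast to BP_玩家控制器.
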(event EventPostLogin
  (params (NewPlayer :type Player%20Controller%20Object%20Reference))
  (bind _asbp_大廳玩家控制器 (Utilities|Casting|CastToBP_大廳玩家控制器 NewPlayer))
  (Utilities|Array|AddUnique (Variables|Default|Get所有玩家控制器) _asbp_大廳玩家控制器))

(event EventOnLogout
  (params (ExitingController :type Controller%20Object%20Reference))
  (bind _asbp_大廳玩家控制器 (Utilities|Casting|CastToBP_大廳玩家控制器 ExitingController))
  (Utilities|Array|RemoveItem (Variables|Default|Get所有玩家控制器) _asbp_大廳玩家控制器)
  (bind _asbp_大廳玩家控制器_2 (Utilities|Casting|CastToBP_大廳玩家控制器 (Game|GetPlayerController 0)))
  (Default|更新玩家資訊介面 _asbp_大廳玩家控制器_2))

(fn ConstructionScript)

(fn 透過編號尋找玩家控制器
  (params (B :type String))
  (for _array_element (Variables|Default|Get所有玩家控制器)
    (bind _asbp_玩家控制器 (Utilities|Casting|CastToBP_玩家控制器 (Pawn|GetControlledPawn _array_element)))
    (if (Utilities|Enum|Equal(Enum) (Variables|/Game/BP/BP_玩家控制器.BP_玩家控制器_C|Get玩家代號 _asbp_玩家控制器) B)
      (return _array_element))))