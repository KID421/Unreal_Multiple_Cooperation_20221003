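; Lobby player controller for a multiplayer session, managing the lobby UI, player roster and leaving the room.
; On local BeginPlay it shows BW_大廳主要介面 and calls CE生成玩家, which possesses a new BP_玩家控制器 pawn carrying the GameInstance name and a timestamp-built ID.
; 更新玩家資訊介面 then gathers names and IDs through the GameMode and pushes them to every controller's widget.
; Other events set the GameState map number or destroy the session and open the start level.
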(event Custom|CE%20生成玩家
  (params (玩家名稱 :type Text))
  (bind _returnvalue (Math|DateTime|Now))
  (bind _returnvalue_2 (Actor|GetActorOfClass "/Script/Engine.PlayerStart"))
  (bind _returnvalue_3 (Game|SpawnActorfromClass "/Game/BP/BP_玩家控制器.BP_玩家控制器_C" (Transformation|GetActorTransform _returnvalue_2) "Undefined" 0 玩家名稱 (Utilities|String|Append (Utilities|String|ToString(Integer) (.year _returnvalue)) (Utilities|String|ToString(Integer) (.month _returnvalue)) (Utilities|String|ToString(Integer) (.day _returnvalue)) (Utilities|String|ToString(Integer) (.hour _returnvalue)) (Utilities|String|ToString(Integer) (.minute _returnvalue)) (Utilities|String|ToString(Integer) (.second _returnvalue)) (Utilities|String|ToString(Integer) (.millisecond _returnvalue))) 0))
  (Pawn|Possess _returnvalue_3)
  (CallFunction|更新玩家資訊介面))

(event Custom|伺服器更新地圖
  (params (地圖編號 :type Integer))
  (bind _asbp_大廳遊戲狀態 (Utilities|Casting|CastToBP_大廳遊戲狀態 (Game|GetGameState)))
  (Variables|/Game/BP/BP_大廳遊戲狀態.BP_大廳遊戲狀態_C|Set地圖編號 _asbp_大廳遊戲狀態 地圖編號))

(event Custom|客戶端更新玩家資訊
  (params (玩家名稱陣列 :type Array%20of%20Texts) (玩家編號陣列 :type Array%20of%20Strings))
  (Default|更新玩家清單 (Variables|Default|GetBW%20大廳主要介面) 玩家名稱陣列 玩家編號陣列))

(event Custom|客戶端退出房間
  (|DestroySession self
    (:OnSuccess
      (Game|OpenLevel(byObjectReference) "/Game/地圖/開始畫面.開始畫面"))))

(event EventBeginPlay
  (if (Pawn|IsLocalController)
    (bind _returnvalue (UserInterface|CreateWidget "/Game/BP/BW_大廳主要介面.BW_大廳主要介面_C" self))
    (UserInterface|Viewport|AddtoViewport _returnvalue 0)
    (Variables|Default|SetBW%20大廳主要介面 _returnvalue)
    (Variables|Default|SetbShowMouseCursor true)
    (bind _asgi_遊戲實體物件 (Utilities|Casting|CastToGI_遊戲實體物件 (Game|GetGameInstance)))
    (CallFunction|CE生成玩家 (Variables|/Game/BP/GI_遊戲實體物件.GI_遊戲實體物件_C|Get玩家名稱 _asgi_遊戲實體物件))))

(fn ConstructionScript)

(fn 更新玩家資訊介面
  (Utilities|Array|Clear (Variables|Default|Get玩家名稱陣列))
  (Utilities|Array|Clear (Variables|Default|Get玩家代號陣列))
  (for _array_element (Variables|/Game/BP/BP_大廳遊戲模式.BP_大廳遊戲模式_C|Get所有玩家控制器 (.AsBP%20大廳遊戲模式 (Utilities|Casting|CastToBP_大廳遊戲模式 (Game|GetGameMode))))
    (bind _asbp_玩家控制器 (Utilities|Casting|CastToBP_玩家控制器 (Pawn|GetControlledPawn _array_element)))
    (Utilities|Array|Add (Variables|Default|Get玩家名稱陣列) (Variables|/Game/BP/BP_玩家控制器.BP_玩家控制器_C|Get玩家名稱 _asbp_玩家控制器))
    (Utilities|Array|Add (Variables|Default|Get玩家代號陣列) (Variables|/Game/BP/BP_玩家控制器.BP_玩家控制器_C|Get玩家代號 _asbp_玩家控制器)))
  (for _array_element_2 (Variables|/Game/BP/BP_大廳遊戲模式.BP_大廳遊戲模式_C|Get所有玩家控制器 (.AsBP%20大廳遊戲模式 (Utilities|Casting|CastToBP_大廳遊戲模式 (Game|GetGameMode))))
    (CallFunction|客戶端更新玩家資訊 _array_element_2 (Variables|Default|Get玩家名稱陣列) (Variables|Default|Get玩家代號陣列))))